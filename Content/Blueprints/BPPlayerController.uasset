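; Player controller for cursor-driven scene interaction, with a context menu, object selection and hold-to-navigate camera input.
; Holding right mouse enables move and look input, while a quick click opens the ContextMenu widget at the cursor.
; Left-click release line-traces from the deprojected cursor, storing and printing SelectedObject.
; F only prints a text-file dialog result; TransformEditor creation and updates are disconnected, and TracePosition is an uncalled helper here.
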(event EventBeginPlay
  (bind _returnvalue (UserInterface|CreateWidget "/Game/Blueprints/ContextMenu.ContextMenu_C"))
  (bind _output_get (Variables|Default|SetContextMenu _returnvalue))
  (UserInterface|Viewport|AddtoViewport _output_get -1)
  (Input|SetIgnoreMoveInput true)
  (Input|SetIgnoreLookInput true)
  (Input|SetInputModeGameandUI self _returnvalue "DoNotLock" true))

(event EventTick
  (params (DeltaSeconds :type Float%20%28single-precision%29)))

(event Input|MouseEvents|RightMouseButton
  (params (Key :type Key%20Structure :default "None"))
  (:Pressed
    (Input|SetIgnoreMoveInput false)
    (Input|SetIgnoreLookInput false)
    (bind _returnvalue (Class|WidgetLayoutLibrary|GetMousePositiononViewport))
    (Variables|Default|SetLastTimeClicked (Utilities|Time|GetRealTimeSeconds))
    (Variables|Default|SetClickedMousePosition _returnvalue))
  (:Released
    (Input|SetIgnoreMoveInput true)
    (Input|SetIgnoreLookInput true)
    (if (<= (- (Utilities|Time|GetRealTimeSeconds) (Variables|Default|GetLastTimeClicked)) 0.15)
      (Default|ShowContextMenu (Variables|Default|GetContextMenu) _returnvalue))))

(event Input|MouseEvents|LeftMouseButton
  (params (Key :type Key%20Structure :default "None"))
  (:Released
    (bind _returnvalue (Class|WidgetLayoutLibrary|GetMousePositiononViewport))
    (bind _hitactor (CallFunction|TraceObject _returnvalue))
    (Development|PrintString (Utilities|GetDisplayName _hitactor))
    (bind _output_get (Variables|Default|SetSelectedObject _hitactor))))

(event Input|KeyboardEvents|F
  (params (Key :type Key%20Structure :default "None"))
  (:Pressed
    (bind _returnvalue (Class|FileDialogsBPLibrary|OpenFileDialog (Utilities|Array|MakeArray "*.txt") "Text file"))
    (Development|PrintString _returnvalue)))

(fn ConstructionScript)

(fn TracePosition
  (params (ViewportPosition :type Vector%202D%20Structure%20%28by%20ref%29))
  (bind (_x _y) (Math|Vector2D|BreakVector2D ViewportPosition))
  (bind _maxdistance (LocalVariables|GetMaxDistance))
  (bind (_worldlocation _worlddirection) (Class|PlayerController|DeprojectScreenPositiontoWorld _x _y))
  (bind _returnvalue (* _worlddirection _maxdistance))
  (bind _returnvalue_2 (+ _worldlocation _returnvalue))
  (bind (_outhit _returnvalue_3) (Collision|LineTraceByChannel _worldlocation _returnvalue_2 "TraceTypeQuery1" false 0 "None"))
  (if _returnvalue_3
    (return (.Location (Collision|BreakHitResult _outhit)))
    (else
      (return _returnvalue_2))))

(fn TraceObject
  (params (ViewportPosiition :type Vector%202D%20Structure))
  (bind (_x _y) (Math|Vector2D|BreakVector2D ViewportPosiition))
  (bind (_worldlocation _worlddirection) (Class|PlayerController|DeprojectScreenPositiontoWorld _x _y))
  (bind (_outhit _returnvalue) (Collision|LineTraceByChannel _worldlocation (+ _worldlocation (* _worlddirection (LocalVariables|GetMaxDistance))) "TraceTypeQuery1" false 0 "None"))
  (if _returnvalue
    (return (.HitActor (Collision|BreakHitResult _outhit)))))